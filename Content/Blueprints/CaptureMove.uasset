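; Clickable capture-move marker for a quantum chess-style board game, destroying itself if nothing lies beneath it or it overlaps anything other than its Victim.
; On click, an uncertain selected piece is measured through BP_Board's qubits, and absence just passes the turn.
; Otherwise the victim's square is measured, removing the victim and resetting its qubit if present.
; The attacker then moves there via the player character, which clears moves and changes turns.
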(event `self.ReceiveBeginPlay`
  (bind _asplayer_ (cast `/Game/Blueprints/GlobalBP/Player+` (`GameplayStatics.GetPlayerCharacter` 0)))
  (set `self.Character` _asplayer_)
  (bind _outactors (`GameplayStatics.GetAllActorsOfClass` "/Game/Blueprints/BP_Board.BP_Board_C"))
  (bind _output (`|GetArrayItem` _outactors))
  (if (`KismetSystemLibrary.IsValid` _output)
    (set `self.Board` _output)))

(event `self.ReceiveActorBeginOverlap`
  (params (OtherActor :type "Actor Object Reference"))
  (if (`KismetSystemLibrary.IsValid` self)
    (bind _asbp_piece (cast `/Game/Blueprints/BP_Piece` OtherActor)
      (:`then`
        (if (not (== _asbp_piece (`self.Victim`)))
          (`self.K2_DestroyActor` :!label _label)))
      (:`CastFailed`
        (goto _label)))))

(event `self.ReceiveActorOnClicked`
  (params (ButtonPressed :type "Key Structure"))
  (bind (_returnvalue_x _returnvalue_y) (`KismetMathLibrary.BreakVector` (`self.K2_GetActorLocation`)))
  (bind _board (`self.Board`))
  (bind _character (`self.Character`))
  (bind _board_2 (`self.Board`))
  (bind _victim (`self.Victim`))
  (bind _board_3 (`self.Board`))
  (bind _character_2 (`self.Character`))
  (bind (_returnvalue_x_2 _returnvalue_y_2) (`KismetMathLibrary.BreakVector` (`self.K2_GetActorLocation` (`self.Victim`))))
  (bind (_returnvalue_x_3 _returnvalue_y_3) (`KismetMathLibrary.BreakVector` (`self.K2_GetActorLocation` _victim)))
  (bind _asbp_piece (cast `/Game/Blueprints/BP_Piece` _victim :!pure true))
  (bind _selected_piece (`/Game/Blueprints/GlobalBP/Player+.Selected Piece` _character))
  (bind (_returnvalue_x_4 _returnvalue_y_4) (`KismetMathLibrary.BreakVector` (`self.K2_GetActorLocation` _selected_piece)))
  (bind (_returnvalue_x_5 _returnvalue_y_5) (`KismetMathLibrary.BreakVector` (`self.K2_GetActorLocation` (`/Game/Blueprints/GlobalBP/Player+.Selected Piece` (`self.Character`)))))
  (`GameplayStatics.PlaySound2D` "/Engine/VREditor/Sounds/VR_ungrab.VR_ungrab" 1.0 1.0 0.0 null null)
  (if (`KismetMathLibrary.NearlyEqual_FloatFloat` (`/Game/Blueprints/BP_Piece.Probability` _selected_piece) 1.0 1e-05)
    (bind _qubit (`/Game/Blueprints/GlobalBP/Player+.Get Qubit` (`self.Character`) _returnvalue_x_2 _returnvalue_y_2 :!label _label_2))
    (set `/Game/Blueprints/BP_Board.Measure` _qubit _board_2)
    (`/Game/Blueprints/BP_Board.Measurement` _board_2)
    (if (`/Game/Blueprints/BP_Board.MeasurementResult` _board_2)
      (`KismetSystemLibrary.PrintString` "Victim Present" true true (struct :`R` 1.0 :`G` 0.07426 :`A` 1.0) 10.0)
      (if (`KismetSystemLibrary.IsValid` _victim)
        (bind _qubit_2 (`/Game/Blueprints/GlobalBP/Player+.Get Qubit` (`self.Character`) _returnvalue_x_3 _returnvalue_y_3))
        (set `/Game/Blueprints/BP_Board.ResetQubit` _qubit_2 _board_3)
        (`/Game/Blueprints/BP_Board.Reset Qubit` _board_3)
        (set `/Game/Blueprints/BP_Piece.Probability` 0.0 _asbp_piece)
        (if (`KismetSystemLibrary.IsValid` _asbp_piece)
          (`self.K2_DestroyActor` _asbp_piece)
          (bind _qubit_3 (`/Game/Blueprints/GlobalBP/Player+.Get Qubit` (`self.Character`) _returnvalue_x_5 _returnvalue_y_5 :!label _label_3))
          (set `/Game/Blueprints/BP_Board.Source` _qubit_3 (`self.Board`))
          (bind _qubit_4 (`/Game/Blueprints/GlobalBP/Player+.Get Qubit` _character_2 _returnvalue_x _returnvalue_y))
          (set `/Game/Blueprints/BP_Board.Target` _qubit_4 (`self.Board`))
          (`/Game/Blueprints/GlobalBP/Player+.Normal Move S` _character_2 _returnvalue_x _returnvalue_y)
          (`/Game/Blueprints/GlobalBP/Player+.Clear Moves` (`self.Character`))
          (`GameplayStatics.PlaySound2D` "/Engine/VREditor/Sounds/UI/Object_Snaps_To_Grid.Object_Snaps_To_Grid" 1.0 1.0 0.0 null null)
          (`/Game/Blueprints/GlobalBP/Player+.ChangeTurns` (`self.Character`) :!label _label_4))
        (else
          (goto _label_4)))
      (else
        (`KismetSystemLibrary.PrintString` "Victim Not there" true true (struct :`G` 1.0 :`B` 0.162547 :`A` 1.0) 10.0)
        (goto _label_3)))
    (else
      (bind _qubit_5 (`/Game/Blueprints/GlobalBP/Player+.Get Qubit` _character _returnvalue_x_4 _returnvalue_y_4))
      (set `/Game/Blueprints/BP_Board.Measure` _qubit_5 _board)
      (`/Game/Blueprints/BP_Board.Measurement` _board)
      (if (`/Game/Blueprints/BP_Board.MeasurementResult` _board)
        (goto _label_2)
        (else
          (goto _label_4))))))

(event `self.ReceiveTick`
  (params (DeltaSeconds :type "Float (single-precision)")))

(fn `UserConstructionScript`
  (bind _returnvalue (`self.K2_GetActorLocation`))
  (bind (_outhit _returnvalue_2) (`KismetSystemLibrary.LineTraceSingle` _returnvalue (+ _returnvalue (* (`self.GetActorUpVector`) -50.0)) "TraceTypeQuery1"))
  (if _returnvalue_2
    _
    (elif (`KismetSystemLibrary.IsValid` self)
      (`self.K2_DestroyActor`))))