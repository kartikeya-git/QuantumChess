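; Clickable move marker for a qubit-based board game that resolves a move onto an obstacle's square by quantum measurement.
; On click, the Board measures the selected piece's qubit, zeroing its probability and ending the turn if absent, otherwise measuring the obstacle's qubit.
; A present obstacle just passes the turn, while an absent one is destroyed and the piece moves there.
; The marker self-destroys on overlap or when its construction-time downward trace hits nothing.
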(event `self.ReceiveBeginPlay`
  (bind _asplayer_ (cast `/Game/Blueprints/GlobalBP/Player+` (`GameplayStatics.GetPlayerCharacter` 0)))
  (bind _output_get (set `self.Character` _asplayer_))
  (set `self.Board` (`/Game/Blueprints/GlobalBP/Player+.Board` _output_get)))

(event `self.ReceiveActorBeginOverlap`
  (params (OtherActor :type "Actor Object Reference"))
  (if (`KismetSystemLibrary.IsValid` self)
    (`self.K2_DestroyActor`)))

(event `self.ReceiveActorOnClicked`
  (params (ButtonPressed :type "Key Structure"))
  (bind (_loc_x _loc_y) (`KismetMathLibrary.BreakVector2D` (`self.Loc`)))
  (bind _character (`self.Character`))
  (bind _character_2 (`self.Character`))
  (bind _board (`self.Board`))
  (bind _board_2 (`self.Board`))
  (bind _character_3 (`self.Character`))
  (bind _obstacle (`self.Obstacle`))
  (bind (_returnvalue_x _returnvalue_y) (`KismetMathLibrary.BreakVector` (`self.K2_GetActorLocation` (`self.Obstacle`))))
  (bind _selected_piece (`/Game/Blueprints/GlobalBP/Player+.Selected Piece` _character_2))
  (bind (_returnvalue_x_2 _returnvalue_y_2) (`KismetMathLibrary.BreakVector` (`self.K2_GetActorLocation` _selected_piece)))
  (bind _qubit (`/Game/Blueprints/GlobalBP/Player+.Get Qubit` _character_2 _returnvalue_x_2 _returnvalue_y_2))
  (set `/Game/Blueprints/BP_Board.Measure` _qubit _board_2)
  (set `/Game/Blueprints/BP_Board.Source` _qubit _board_2)
  (`/Game/Blueprints/BP_Board.Measurement` _board_2)
  (if (`/Game/Blueprints/BP_Board.MeasurementResult` _board_2)
    (set `self.Loc` (`KismetMathLibrary.MakeVector2D` _returnvalue_x _returnvalue_y))
    (bind _qubit_2 (`/Game/Blueprints/GlobalBP/Player+.Get Qubit` _character_3 _returnvalue_x _returnvalue_y))
    (set `/Game/Blueprints/BP_Board.Measure` _qubit_2 _board)
    (set `/Game/Blueprints/BP_Board.Target` _qubit_2 _board)
    (`/Game/Blueprints/BP_Board.Measurement` _board)
    (if (`/Game/Blueprints/BP_Board.MeasurementResult` _board)
      (`/Game/Blueprints/GlobalBP/Player+.ChangeTurns` _character)
      (else
        (if (`KismetSystemLibrary.IsValid` _obstacle)
          (`self.K2_DestroyActor` _obstacle))
        (`/Game/Blueprints/GlobalBP/Player+.Normal Move S` _character _loc_x _loc_y)
        (`/Game/Blueprints/GlobalBP/Player+.ChangeTurns` _character)))
    (else
      (set `/Game/Blueprints/BP_Piece.Probability` 0.0 _selected_piece)
      (if (`KismetSystemLibrary.IsValid` _selected_piece)
        (`self.K2_DestroyActor`)
        (`/Game/Blueprints/GlobalBP/Player+.ChangeTurns` _character_3)))))

(fn `UserConstructionScript`
  (bind _returnvalue (`self.K2_GetActorLocation`))
  (bind (_outhit _returnvalue_2) (`KismetSystemLibrary.LineTraceSingle` _returnvalue (+ _returnvalue (* (`self.GetActorUpVector`) -50.0)) "TraceTypeQuery1"))
  (if _returnvalue_2
    _
    (elif (`KismetSystemLibrary.IsValid` self)
      (`self.K2_DestroyActor`))))