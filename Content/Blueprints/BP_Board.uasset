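; Quantum chess board actor that bridges piece moves to Qiskit functions through a Python component, arranging the board and reading probabilities on BeginPlay.
; Events run quantum moves (sqrt-iSwap), normal moves (iSwap), measurement, qubit resets and probability queries.
; Normal moves record obstacle qubits, choosing a slide for blocked non-Knight, non-Pawn pieces and a jump otherwise.
; CreatePiece spawns a copy of the selected piece at the previous location when Slide is set.
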(event `self.ReceiveBeginPlay`
  ;[1 1 1] Begin Play
  ;;[0 0 0] Set Character reference
  (bind _asplayer_ (cast `/Game/Blueprints/GlobalBP/Player+` (`GameplayStatics.GetPlayerCharacter` 0)))
  (set `self.Character` _asplayer_)
  (`PythonComponent.CallPythonComponentMethod` (`self.Python`) "arrange" "")
  (`self.Get Prob`) ; Initialize Prob
)

(event `Quantum Move`
  ;[1 1 1] Call to Python, Qiskit Functions
  ;;[0.724 0 1] Do sqrt of iSwap on Source and Target
  (`PythonComponent.CallPythonComponentMethod` (`self.Python`) "quantumm_move" "")
  (`KismetSystemLibrary.PrintString` "Quantum Move"))

(event `Get Prob`
  ;[1 1 1] Call to Python, Qiskit Functions
  ;;[1 0.6759 0] Get all probabilities
  (bind _output_strings (`PythonComponent.CallPythonComponentMethodStringArray` (`self.Python`) "get_probability" ""))
  (set `self.Probability Strings` _output_strings))

(event `Normal Move`
  (bind _python (`self.Python`))
  ;[1 1 1] Do iSwap on Source and Target
  (`KismetArrayLibrary.Array_Clear` (`self.P`))
  (if (!= (`KismetArrayLibrary.Array_Length` (`self.Obstacles`)) 0)
    (for _array_element (`self.Obstacles`)
      (bind (_returnvalue_x _returnvalue_y) (`KismetMathLibrary.BreakVector` (`self.K2_GetActorLocation` _array_element)))
      (bind _qubit (`/Game/Blueprints/GlobalBP/Player+.Get Qubit` (`self.Character`) _returnvalue_x _returnvalue_y))
      (`KismetArrayLibrary.Array_AddUnique` (`self.P`) (`KismetStringLibrary.Conv_IntToString` _qubit)))
    (if (select `/Game/Blueprints/Enums/PieceType` (`/Game/Blueprints/BP_Piece.Piece Type` (`/Game/Blueprints/GlobalBP/Player+.Selected Piece` (`self.Character`))) :`NewEnumerator4` true :`NewEnumerator7` true :`NewEnumerator8` true :`NewEnumerator9` true)
      (`PythonComponent.CallPythonComponentMethod` _python "slide_move" "")
      (`KismetSystemLibrary.PrintString` "Slide Move")
      (set `self.Slide` true)
      (else
        (`PythonComponent.CallPythonComponentMethod` _python "normal_move" "" :!label _label)
        (`KismetSystemLibrary.PrintString` "Jump Move")))
    (else
      (goto _label))))

(event `Reset Qubit`
  ;[1 1 1] Call to Python, Qiskit Functions
  ;;[0 0 0] Reset Qubit to 0
  (`PythonComponent.CallPythonComponentMethod` (`self.Python`) "reset_qubit" ""))

(event `Measurement`
  ;[1 1 1] Call to Python, Qiskit Functions
  ;;[1 0.7698 0] DO measurement on single qubit
  (bind _returnvalue (`PythonComponent.CallPythonComponentMethodBool` (`self.Python`) "measure" ""))
  (set `self.MeasurementResult` _returnvalue))

(event `Reset Qubit1`
  ;[1 1 1] Call to Python, Qiskit Functions
  ;;[0 0 0] Reset Qubit to 1
  (`PythonComponent.CallPythonComponentMethod` (`self.Python`) "reset_qubit1" ""))

(fn `Create Piece`
  (bind (_prevlocation_x _prevlocation_y) (`KismetMathLibrary.BreakVector` (`self.PrevLocation`)))
  (bind _selected_piece (`/Game/Blueprints/GlobalBP/Player+.Selected Piece` (`self.Character`)))
  (if (`self.Slide`)
    (`|SpawnActorFromClass` "/Game/Blueprints/BP_Piece.BP_Piece_C" (`KismetMathLibrary.MakeTransform` (`KismetMathLibrary.MakeVector` _prevlocation_x _prevlocation_y 60.0)) "Undefined" "OverrideRootScale" null (`/Game/Blueprints/BP_Piece.Piece Color` _selected_piece) (`/Game/Blueprints/BP_Piece.Piece Type` _selected_piece) (`/Game/Blueprints/BP_Piece.Piece Number` _selected_piece) null))
  (return))

(fn `UserConstructionScript`)