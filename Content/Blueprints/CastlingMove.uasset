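; Clickable castling-move marker for a quantum chess game, which destroys itself on actor overlap.
; On click, it line-traces to either side, with color-dependent distances, for a same-color, presumed rook with FirstMove set.
; It moves that piece to the midpoint between king and marker and the king onto the marker, then changes turns.
; SwapQubits mirrors each move on BP_Board by setting source and target qubits and calling NormalMove.
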(event `self.ReceiveActorBeginOverlap`
  (params (OtherActor :type "Actor Object Reference"))
  (if (`KismetSystemLibrary.IsValid` self)
    (`self.K2_DestroyActor`)))

(event `self.ReceiveBeginPlay`
  (bind _asplayer_ (cast `/Game/Blueprints/GlobalBP/Player+` (`GameplayStatics.GetPlayerCharacter` 0)))
  (set `self.Character` _asplayer_)
  (bind _outactors (`GameplayStatics.GetAllActorsOfClass` "/Game/Blueprints/BP_Board.BP_Board_C"))
  (bind _output (`|GetArrayItem` _outactors))
  (if (`KismetSystemLibrary.IsValid` _output)
    (set `self.Board` _output)))

(event `self.ReceiveActorOnClicked`
  (params (ButtonPressed :type "Key Structure"))
  (`GameplayStatics.PlaySound2D` "/Engine/VREditor/Sounds/VR_ungrab.VR_ungrab" 1.0 1.0 0.0 null null)
  (`self.Castle`)
  (`/Game/Blueprints/GlobalBP/Player+.ChangeTurns` (`self.Character`)))

(fn `UserConstructionScript`)